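; Interactive swinging door that opens away from the player, closes automatically when they leave its trigger, and plays a locked sound when not openable.
; The Action input toggles it if the player is inside the trigger, looking at its box, and the door is available.
; FCheckPlayerPosition picks the swing direction by comparing positions for four axis-aligned yaws.
; A timeline lerps the rotation, reversing to close.
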(event OnComponentBeginOverlap(TriggerDoor)
  (params (OtherActor :type Actor%20Object%20Reference) (OtherComp :type Primitive%20Component%20Object%20Reference) (OtherBodyIndex :type Integer) (bFromSweep :type Boolean) (SweepResult :type Hit%20Result%20Structure%20%28by%20ref%29))
  ;[1 1 1] Check if player inside
  (if (== OtherActor (Game|Player|GetPlayerPawn 0))
    (Variables|Default|SetisPlayerInTrigger true)))

(event OnComponentEndOverlap(TriggerDoor)
  (params (OtherActor :type Actor%20Object%20Reference) (OtherComp :type Primitive%20Component%20Object%20Reference) (OtherBodyIndex :type Integer))
  ;[1 1 1] Check if player inside
  (if (== (Game|Player|GetPlayerPawn 0) OtherActor)
    (Variables|Default|SetisPlayerInTrigger false)
    (if (Variables|Default|GetisDoorOpen)
      (Variables|Default|SetisDoorOpen false)
      ;[1 1 1] Test for Door
      (Audio|PlaySoundatLocation "/Game/Sounds/SoundCue_Door_Close.SoundCue_Door_Close" (Transformation|GetActorLocation))
      (bind _rotation (Timeline|Timeline_0 Reverse)
        (:Update
          (Transformation|SetRelativeRotation (Variables|Default|GetSceneComponent) (Math|Rotator|Lerp(Rotator) "0,0.000000, 0" (Variables|Default|GetdoorLerpVector) _rotation true) false))
        (:Finished
          (Variables|Default|SetisDoorAvailable true))))))

(event EventBeginPlay
  ;[1 1 1] Enable input on play
  (Input|EnableInput (Game|GetPlayerController 0)))

(event Input|ActionEvents|InputActionAction
  (bind _returnvalue (Transformation|GetActorLocation))
  ;[1 1 1] Test for Door
  (:Pressed
    (if (Variables|Default|GetisPlayerInTrigger)
      (bind _asplayer (Utilities|Casting|CastToPlayer (Game|Player|GetPlayerPawn 0)))
      (bind _islooking (Default|CheckifLookingat _asplayer (Variables|Default|GetBox)))
      (if _islooking
        (if (Variables|Default|GetisDoorAvailable)
          (if (Variables|Default|GetisOpenable)
            (if (Variables|Default|GetisDoorOpen)
              (Variables|Default|SetisDoorOpen false)
              (Variables|Default|SetisDoorAvailable false)
              (Audio|PlaySoundatLocation "/Game/Sounds/SoundCue_Door_Close.SoundCue_Door_Close" _returnvalue)
              (bind _rotation (Timeline|Timeline_0 Reverse)
                (:Update
                  (Transformation|SetRelativeRotation (Variables|Default|GetSceneComponent) (Math|Rotator|Lerp(Rotator) "0,0.000000, 0" (Variables|Default|GetdoorLerpVector) _rotation true) false))
                (:Finished
                  (Variables|Default|SetisDoorAvailable true)))
              (else
                (Variables|Default|SetisDoorOpen true)
                (Variables|Default|SetisDoorAvailable false)
                (CallFunction|FCheckPlayerPosition)
                (Audio|PlaySoundatLocation "/Game/Sounds/SoundCue_Door_Open.SoundCue_Door_Open" _returnvalue)
                (Timeline|Timeline_0 Play)))
            (else
              (Variables|Default|SetisDoorAvailable false)
              (Audio|PlaySoundatLocation "/Game/Audio/SFXDoorLocked01.SFXDoorLocked01" (Transformation|GetActorLocation))
              (Utilities|FlowControl|Delay 0.0)
              (Variables|Default|SetisDoorAvailable true))))))))

(fn ConstructionScript)

(fn FCheckPlayerPosition
  (bind _output_get (Variables|Default|SetdoorWorldRotation (Transformation|GetWorldRotation (Variables|Default|GetScene))))
  (if (Math|Rotator|Equal(Rotator) _output_get "0.000000, 0, 0" 2.0)
    ;[1 1 1] ROT = 0
    (if (> (.X (Math|Vector|BreakVector (Transformation|GetWorldLocation (Variables|Default|GetScene)))) (.X (Math|Vector|BreakVector (Transformation|GetActorLocation (Game|Player|GetPlayerPawn 0)))))
      (Variables|Default|SetisPlayerInFront true)
      (Variables|Default|SetdoorLerpVector "0,90.000000, 0")
      (else
        (Variables|Default|SetisPlayerInFront false)
        (Variables|Default|SetdoorLerpVector "0,-90.000000, 0")))
    (elif (Math|Rotator|Equal(Rotator) _output_get "0.000000,90.000000, 0" 2.0)
      ;[1 1 1] ROT = 90
      (if (> (.Y (Math|Vector|BreakVector (Transformation|GetWorldLocation (Variables|Default|GetScene)))) (.Y (Math|Vector|BreakVector (Transformation|GetActorLocation (Game|Player|GetPlayerPawn 0)))))
        (Variables|Default|SetisPlayerInFront true)
        (Variables|Default|SetdoorLerpVector "0,90.000000, 0")
        (else
          (Variables|Default|SetisPlayerInFront false)
          (Variables|Default|SetdoorLerpVector "0,-90.000000, 0")))
      (elif (Math|Rotator|Equal(Rotator) _output_get "0.000000,180.000000, 0" 2.0)
        ;[1 1 1] ROT = 180
        (if (< (.X (Math|Vector|BreakVector (Transformation|GetWorldLocation (Variables|Default|GetScene)))) (.X (Math|Vector|BreakVector (Transformation|GetActorLocation (Game|Player|GetPlayerPawn 0)))))
          (Variables|Default|SetisPlayerInFront true)
          (Variables|Default|SetdoorLerpVector "0,90.000000, 0")
          (else
            (Variables|Default|SetisPlayerInFront false)
            (Variables|Default|SetdoorLerpVector "0,-90.000000, 0")))
        (elif (Math|Rotator|Equal(Rotator) _output_get "0.000000,270.000000, 0" 2.0)
          ;[1 1 1] ROT = 270
          (if (< (.Y (Math|Vector|BreakVector (Transformation|GetWorldLocation (Variables|Default|GetScene)))) (.Y (Math|Vector|BreakVector (Transformation|GetActorLocation (Game|Player|GetPlayerPawn 0)))))
            (Variables|Default|SetisPlayerInFront true)
            (Variables|Default|SetdoorLerpVector "0,90.000000, 0")
            (else
              (Variables|Default|SetisPlayerInFront false)
              (Variables|Default|SetdoorLerpVector "0,-90.000000, 0"))))))))