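; Player character Blueprint that handles movement, camera look and an inspect mode for examining objects, and adds the game UI on begin play.
; ExamineObject locks controls, snaps the object to an attachment point and switches to a second camera, where look axes rotate the object instead.
; ReleaseObject restores the object, camera and controls.
; CheckifLookingAt line-traces from the camera to test for a given component; CamDropper holds only unconnected camera logic.
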(event Custom|ForceSpeedNull
  ;[1 1 1] Nullify speed
  (Variables|/Script/Engine.MovementComponent|SetVelocity (Variables|Character|GetCharacterMovement) "0, 0, 0"))

(event EventBeginPlay
  ;[1 1 1] Begin Play - Add UI Widget
  (bind _returnvalue (UserInterface|CreateWidget "/Game/UI/GameUIWidget.GameUIWidget_C"))
  (Variables|Default|SetGameWidget _returnvalue)
  (UserInterface|Viewport|AddtoViewport 0))

(event Input|AxisEvents|InputAxisForward_Backward
  (params (AxisValue :type Float%20%28single-precision%29))
  ;[1 1 1] Movement
  (if (Variables|Default|GetisControllable)
    (Pawn|Input|AddMovementInput (Transformation|GetActorForwardVector) AxisValue false)
    (if (or (!= AxisValue 0.0) (!= 0.0 (stale Input|AxisEvents|InputAxisLeft_Right AxisValue)))
      (Variables|Default|SetisMoving true)
      (else
        (Variables|Default|SetisMoving false)))))

(event Input|AxisEvents|InputAxisLeft_Right
  (params (AxisValue :type Float%20%28single-precision%29))
  ;[1 1 1] Movement
  (if (Variables|Default|GetisControllable)
    (Pawn|Input|AddMovementInput (Transformation|GetActorRightVector) AxisValue false)
    (if (or (!= (stale Input|AxisEvents|InputAxisForward_Backward AxisValue) 0.0) (!= 0.0 AxisValue))
      (Variables|Default|SetisMoving true)
      (else
        (Variables|Default|SetisMoving false)))))

(event Input|AxisEvents|InputAxisRotate_Left_Right
  (params (AxisValue :type Float%20%28single-precision%29))
  (bind _objectexamined (Variables|Default|GetObjectExamined))
  ;[1 1 1] Camera normal mode
  (Variables|Default|SetcurrentYawValue AxisValue)
  (if (Variables|Default|GetisCameraRotable)
    (if (Variables|Default|GetisSitting)
      _
      (else
        _))
    (Pawn|Input|AddControllerYawInput (* (Variables|Default|GetcamRotFactor) (Variables|Default|GetcurrentYawValue)))
    (if (or (!= (Variables|Default|GetcurrentPitchValue) 0.0) (!= 0.0 (Variables|Default|GetcurrentYawValue)))
      (Variables|Default|SetisCamRotating true)
      (else
        (Variables|Default|SetisCamRotating false)))
    (else
      ;[1 1 1] Camera examine object mode
      (if (Variables|Default|GetcanRotateObject)
        (Transformation|SetWorldRotation _objectexamined (Math|Rotator|CombineRotators (Class|KismetMathLibrary|MakeRot (Variables|Default|GetcurrentYawValue) 0.0 0.0) (Transformation|GetWorldRotation _objectexamined)) false)))))

(event Input|AxisEvents|InputAxisLooking_Up_Down
  (params (AxisValue :type Float%20%28single-precision%29))
  (bind _objectexamined (Variables|Default|GetObjectExamined))
  ;[1 1 1] Camera normal mode
  (Variables|Default|SetcurrentPitchValue AxisValue)
  (if (Variables|Default|GetisCameraRotable)
    (Pawn|Input|AddControllerPitchInput (* (Variables|Default|GetcamRotFactor) (Variables|Default|GetcurrentPitchValue)))
    (else
      ;[1 1 1] Camera examine object mode
      (if (Variables|Default|GetcanRotateObject)
        (Transformation|SetWorldRotation _objectexamined (Math|Rotator|CombineRotators (Transformation|GetWorldRotation _objectexamined) (Class|KismetMathLibrary|MakeRot 0.0 (Variables|Default|GetcurrentPitchValue) 0.0)) false)))))

(fn ConstructionScript)

(fn ExamineObject
  (bind _objectexamined (Variables|Default|GetObjectExamined))
  (Variables|Default|SetisControllable false)
  (Variables|Default|SetisCameraRotable false)
  (Variables|Default|SetexaminedObjectParent (Transformation|GetAttachParent _objectexamined))
  (Class|SceneComponent|Attachto _objectexamined (Variables|Default|GetObjectAttachmentPoint) "None" "SnapToTarget" true)
  (Transformation|SetRelativeTransform (Variables|Default|GetObjectExamined) (Variables|Default|GetexaminedObjectDesiredTransform) false)
  (Components|Activation|SetActive (Variables|Default|GetCamera) false false)
  (Components|Activation|SetActive (Variables|Default|GetCameraExamine) true false)
  (Variables|Default|SetcanRotateObject true))

(fn ReleaseObject
  (bind _objectexamined (Variables|Default|GetObjectExamined))
  (Variables|Default|SetcanRotateObject false)
  (Components|Activation|SetActive (Variables|Default|GetCamera) true false)
  (Components|Activation|SetActive (Variables|Default|GetCameraExamine) false false)
  (Class|SceneComponent|DetachfromParent _objectexamined false)
  (Class|SceneComponent|Attachto _objectexamined (Variables|Default|GetexaminedObjectParent) "None" "SnapToTarget" true)
  (Transformation|SetWorldTransform _objectexamined (Variables|Default|GetexaminedObjectInitOffset) false)
  (Variables|Default|SetisControllable true)
  (Variables|Default|SetisCameraRotable true))

(fn CheckifLookingat
  (params (objectToCheck :type Box%20Component%20Object%20Reference))
  (bind _camera (Variables|Default|GetCamera))
  (bind _returnvalue (Transformation|GetWorldLocation _camera))
  (bind _outhit (Collision|LineTraceByChannel _returnvalue (+ _returnvalue (* (Math|Vector|GetForwardVector _camera) 5e+02)) "TraceTypeQuery1" false 0 "None"))
  (return (== (.HitComponent (Collision|BreakHitResult _outhit)) objectToCheck)))

(fn CamDropper)