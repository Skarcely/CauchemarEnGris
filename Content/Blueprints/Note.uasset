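; Note is an interactable world object that the player can pick up to examine and put back with the Action input.
; A trigger overlap and the Player's look-at check against RaycastCollision gate both the input and the interact prompt.
; Examining hands its SceneComponent, original transform and a fixed display transform to the Player, which handles examine and release.
; Tick updates the prompt only when the look state changes.
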(event OnComponentBeginOverlap(Trigger)
  (params (OtherActor :type Actor%20Object%20Reference) (OtherComp :type Primitive%20Component%20Object%20Reference) (OtherBodyIndex :type Integer) (bFromSweep :type Boolean) (SweepResult :type Hit%20Result%20Structure%20%28by%20ref%29))
  ;[1 1 1] Check if player inside
  (if (== OtherActor (Game|Player|GetPlayerPawn 0))
    (Variables|Default|SetisPlayerInTrigger true)))

(event OnComponentEndOverlap(Trigger)
  (params (OtherActor :type Actor%20Object%20Reference) (OtherComp :type Primitive%20Component%20Object%20Reference) (OtherBodyIndex :type Integer))
  ;[1 1 1] Check if player inside
  (if (== (Game|Player|GetPlayerPawn 0) OtherActor)
    (Variables|Default|SetisPlayerInTrigger false)
    (bind _asplayer (Utilities|Casting|CastToPlayer (Game|Player|GetPlayerPawn 0)))
    (Default|SetInteractVisibility (Variables|/Game/Blueprints/Player.Player_C|GetGameWidget _asplayer) false)))

(event EventBeginPlay
  ;[1 1 1] Enable input on play
  (Input|EnableInput (Game|GetPlayerController 0)))

(event EventTick
  (params (DeltaSeconds :type Float%20%28single-precision%29))
  (bind _returnvalue (Game|Player|GetPlayerPawn 0))
  ;[1 1 1] Check if looking to display interact UI
  (if (not (Variables|Default|GetisBeingExamined))
    (if (Variables|Default|GetisPlayerInTrigger)
      (bind _asplayer (Utilities|Casting|CastToPlayer _returnvalue))
      (bind _islooking (Default|CheckifLookingat _asplayer (Variables|Default|GetRaycastCollision)))
      (bind _output_get (Variables|Default|SetisPlayerLooking _islooking))
      (if (Math|Boolean|NotEqual(Boolean) _output_get (Variables|Default|GetwasPlayerLooking))
        (Variables|Default|SetwasPlayerLooking _output_get)
        (bind _asplayer_2 (Utilities|Casting|CastToPlayer _returnvalue))
        (Default|SetInteractVisibility (Variables|/Game/Blueprints/Player.Player_C|GetGameWidget _asplayer_2) _output_get)))))

(event Input|ActionEvents|InputActionAction
  (bind _returnvalue (Game|Player|GetPlayerPawn 0))
  (bind _scenecomponent (Variables|Default|GetSceneComponent))
  ;[1 1 1] Examine object
  (:Pressed
    (if (Variables|Default|GetisPlayerInTrigger)
      (bind _asplayer (Utilities|Casting|CastToPlayer (Game|Player|GetPlayerPawn 0)))
      (bind _islooking (Default|CheckifLookingat _asplayer (Variables|Default|GetRaycastCollision)))
      (if _islooking
        (if (not (Variables|Default|GetisBusy))
          (if (Variables|Default|GetisBeingExamined)
            (Variables|Default|SetisBeingExamined false)
            (bind _asplayer_2 (Utilities|Casting|CastToPlayer _returnvalue))
            (Default|ReleaseObject _asplayer_2)
            (Variables|Default|SetwasPlayerLooking false)
            (else
              (Variables|Default|SetisBeingExamined true)
              (bind _asplayer_3 (Utilities|Casting|CastToPlayer _returnvalue))
              (Variables|/Game/Blueprints/Player.Player_C|SetObjectExamined _asplayer_3 _scenecomponent)
              (Variables|/Game/Blueprints/Player.Player_C|SetexaminedObjectInitOffset _asplayer_3 (Transformation|GetWorldTransform _scenecomponent))
              (Variables|/Game/Blueprints/Player.Player_C|SetexaminedObjectDesiredTransform _asplayer_3 (Math|Transform|MakeTransform "0, 0, 0" "0.000000,-90.000000,90.000000" "1.000000,1.000000,1.000000"))
              (Default|ExamineObject _asplayer_3)
              (bind _asplayer_4 (Utilities|Casting|CastToPlayer _returnvalue))
              (Default|SetInteractVisibility (Variables|/Game/Blueprints/Player.Player_C|GetGameWidget _asplayer_4) false))))))))

(fn ConstructionScript)