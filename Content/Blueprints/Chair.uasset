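; Chair actor that lets the player sit down and get up with the Action input.
; Sitting requires an empty chair, the player inside the trigger and a look-at check on its raycast collision.
; Two timelines lerp pawn location and control rotation toward sit or stand points, with a busy flag blocking input meanwhile.
; Player movement, camera and collision are disabled and restored around these transitions, and the player's sitting state is updated.
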(event OnComponentBeginOverlap(TriggerChair)
  (params (OtherActor :type Actor%20Object%20Reference) (OtherComp :type Primitive%20Component%20Object%20Reference) (OtherBodyIndex :type Integer) (bFromSweep :type Boolean) (SweepResult :type Hit%20Result%20Structure%20%28by%20ref%29))
  ;[1 1 1] Check if player inside
  (if (== OtherActor (Game|Player|GetPlayerPawn 0))
    (Variables|Default|SetisPlayerInTrigger true)))

(event OnComponentEndOverlap(TriggerChair)
  (params (OtherActor :type Actor%20Object%20Reference) (OtherComp :type Primitive%20Component%20Object%20Reference) (OtherBodyIndex :type Integer))
  ;[1 1 1] Check if player inside
  (if (== (Game|Player|GetPlayerPawn 0) OtherActor)
    (Variables|Default|SetisPlayerInTrigger false)))

(event EventBeginPlay
  ;[1 1 1] Enable input on play
  (Input|EnableInput (Game|GetPlayerController 0)))

(event Input|ActionEvents|InputActionAction
  (bind _returnvalue (Game|GetPlayerController 0))
  (bind _returnvalue_2 (Game|Player|GetPlayerPawn 0))
  (bind _returnvalue_3 (Game|GetPlayerController 0))
  (bind _returnvalue_4 (Game|Player|GetPlayerPawn 0))
  (bind _returnvalue_5 (Game|Player|GetPlayerPawn 0))
  (bind _sitpos (Variables|Default|GetSitPos))
  (bind _standpos (Variables|Default|GetStandPos))
  ;[1 1 1] Tests if able to sit or get up
  (:Pressed
    (if (not (Variables|Default|GetisBusy))
      (if (Variables|Default|GetisChairEmpty)
        (bind _asplayer (Utilities|Casting|CastToPlayer (Game|Player|GetPlayerPawn 0)))
        (bind _islooking (Default|CheckifLookingat _asplayer (Variables|Default|GetRaycastCollision)))
        (if _islooking
          ;[1 1 1] Sit Down
          (if (Variables|Default|GetisPlayerInTrigger)
            (Variables|Default|SetisBusy true)
            (bind _asplayer_2 (Utilities|Casting|CastToPlayer _returnvalue_5))
            (Default|ForceSpeedNull _asplayer_2)
            (bind _asplayer_3 (Utilities|Casting|CastToPlayer _returnvalue_5))
            (Variables|/Game/Blueprints/Player.Player_C|SetisControllable _asplayer_3 false)
            (Variables|/Game/Blueprints/Player.Player_C|SetisCameraRotable _asplayer_3 false)
            (Variables|Default|SetisChairEmpty false)
            (Collision|SetActorEnableCollision _returnvalue_5 false)
            (bind _curve (Timeline|Timeline_0 PlayFromStart)
              (:Update
                (Transformation|SetActorLocation (Game|Player|GetPlayerPawn 0) (Math|Vector|Lerp(Vector) (Transformation|GetActorLocation _returnvalue_5) (Transformation|GetWorldLocation _sitpos) _curve) false)
                (Pawn|SetControlRotation _returnvalue_3 (Math|Rotator|Lerp(Rotator) (Transformation|GetActorRotation _returnvalue_3) (Transformation|GetWorldRotation _sitpos) _curve)))
              (:Finished
                (Variables|Default|SetisBusy false)
                (bind _asplayer_4 (Utilities|Casting|CastToPlayer _returnvalue_5))
                (Variables|/Game/Blueprints/Player.Player_C|SetisCameraRotable _asplayer_4 true)
                (Variables|/Game/Blueprints/Player.Player_C|SetisSitting _asplayer_4 true)))))
        (else
          ;[1 1 1] Get Up
          (Variables|Default|SetisBusy true)
          (bind _asplayer_5 (Utilities|Casting|CastToPlayer _returnvalue_2))
          (Variables|/Game/Blueprints/Player.Player_C|SetisCameraRotable _asplayer_5 false)
          (bind _curve_2 (Timeline|Timeline_1 Play)
            (:Update
              (Transformation|SetActorLocation _returnvalue_4 (Math|Vector|Lerp(Vector) (Transformation|GetActorLocation _returnvalue_2) (Transformation|GetWorldLocation _standpos) _curve_2) false)
              (Pawn|SetControlRotation _returnvalue (Math|Rotator|Lerp(Rotator) (Transformation|GetActorRotation _returnvalue) (Transformation|GetWorldRotation _standpos) _curve_2)))
            (:Finished
              (Variables|Default|SetisBusy false)
              (bind _asplayer_6 (Utilities|Casting|CastToPlayer _returnvalue_2))
              (Variables|/Game/Blueprints/Player.Player_C|SetisControllable _asplayer_6 true)
              (Variables|Default|SetisChairEmpty true)
              (Collision|SetActorEnableCollision _returnvalue_2 true)
              (bind _asplayer_7 (Utilities|Casting|CastToPlayer _returnvalue_4))
              (Variables|/Game/Blueprints/Player.Player_C|SetisSitting _asplayer_7 false)
              (Variables|/Game/Blueprints/Player.Player_C|SetisCameraRotable _asplayer_7 true))))))))

(fn ConstructionScript)